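; An actor component that spawns floating text to show damage received by its owner.
; Its damage event spawns a damage text actor with the value truncated to a whole number, plus a status text actor for critical hits.
; Both actors spawn at the owner's location shifted by a configurable offset, ignoring collisions.
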(event `EventOnDamageReceived`
  (params (DamageTaken :type "Float (double-precision)") (`IsACritHit?` :type Boolean))
  (bind _returnvalue (`self.CalculateSpawnLocation`))
  (`|SpawnActorFromClass` (`self.DamageTextClass`) _returnvalue "AlwaysSpawn" "OverrideRootScale" null (`KismetMathLibrary.FTrunc` DamageTaken) null) ; Spawns an actor to display the damage taken
  (if `IsACritHit?`
    (`|SpawnActorFromClass` (`self.StatusTextClass`) _returnvalue "AlwaysSpawn" "OverrideRootScale" null (`self.StatusText_CriticalHit`) null) ; Spawns an actor to display the critical hit status
  ))

(fn `CalculateSpawnLocation`
  (returns (ReturnValue :type "Transform Structure"))
  (return (`KismetMathLibrary.Conv_VectorToTransform` (+ (`Actor.K2_GetActorLocation` (`self.GetOwner`)) (`self.OwnerSpawnOffset`)))))