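; BP_FloatingText_Parent is the base actor for floating text in the damage display system, animating a scalable text widget.
; On BeginPlay it caches the widget and its scale, then runs a looping timer that updates location and scale.
; Scale grows multiplicatively until a peak check passes, then shrinks, with distance falloff from the player pawn and clamping applied.
; Child classes supply the movement and peak condition.
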(event `self.ReceiveBeginPlay`
  ;[0 1 0 0.5] Initialization Protocols
  (bind _aswidget_scalable_text (cast `/Game/DamageDisplaySystem/UI/Widget_ScalableText` (`WidgetComponent.GetUserWidgetObject` (`self.TextWidget`))))
  (bind _output_get (set `self.ScalableText` _aswidget_scalable_text))
  (set `self.WidgetScale` (`/Game/DamageDisplaySystem/UI/Widget_ScalableText.GetDisplayScale` _output_get)) ; Stores the default scale of the widget
  (`self.RunUpdateCycle`) ; Runs the first update cycle immediately
  (`KismetSystemLibrary.K2_SetTimerDelegate` (delegate `RunUpdateCycle`) (`self.UpdateTimerInterval`) true))

(event `RunUpdateCycle`
  ;[0 1 1 0.5] Updates the floating text state
  (set `self.UpdateIteration` (+ (`self.UpdateIteration`) 1)) ; Updates the timer loop count
  (`self.UpdateWidgetLocation`)
  (`self.UpdateWidgetScale`))

(event `UpdateWidgetLocation`
  ;[0 1 1 0.5] Updates the floating text state
)

(event `UpdateWidgetScale`
  (bind _widgetscale (`self.WidgetScale`))
  ;[0 1 1 0.5] Updates the floating text state
  (bind _output_get (set `self.WidgetScale` (`KismetMathLibrary.SelectFloat` (* _widgetscale (`self.WidgetScaleDecrementPerCycle`)) (* _widgetscale (`self.WidgetScaleIncrementPerCycle`)) (`self.ReachedPointOfMaxWidgetScale?`))))
  (`/Game/DamageDisplaySystem/UI/Widget_ScalableText.SetDisplayScale` (`self.ScalableText`) (`KismetMathLibrary.FClamp` (* _output_get (`self.CalculateDistanceBasedWidgetScaleModifier`)) (`self.MinWidgetScale`) (`self.MaxWidgetScale`))) ; Updates the widget scale
)

(fn `CalculateDistanceBasedWidgetScaleModifier`
  (returns (WidgetScaleModifier :type "Float (double-precision)"))
  ;[0 1 1 0.5] Returns the scale modifier for the widget based on distance from the player
  (return (`KismetMathLibrary.FMax` (- 1.0 (* (`self.GetDistanceTo` (`GameplayStatics.GetPlayerPawn` 0)) (`self.WidgetScaleFallOffPerUnit`))))))

(fn `ReachedPointOfMaxWidgetScale?`
  (returns (`Yes?` :type Boolean))
  ;[1 1 1 0.5] Implemented through child classes
  (return false))

(fn `UserConstructionScript`)