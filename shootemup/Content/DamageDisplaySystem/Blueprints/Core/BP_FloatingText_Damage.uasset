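; Floating damage number actor that shows its damage value in a scalable text widget and flies along a parabolic arc.
; On BeginPlay it sets the text and color, then derives the arc's apex height and per-cycle horizontal step from a starting deviation.
; Each update moves it along the camera's right vector with height from an inverted parabola.
; Horizontal distance covered signals maximum widget scale past the apex and destroys the actor at the arc's end.
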(event EventUpdateWidgetLocation
  (bind _returnvalue (Transformation|GetActorLocation))
  ;[0 1 1 0.5] Updates the floating text state
  (Transformation|SetActorLocation (+ (Math|Vector|MakeVector (.x _returnvalue) (.y _returnvalue) (+ (Variables|RuntimeAllocation|GetMaxHeightInWorldSpace) (* (|(A*(Power(Base,Exp))) (Variables|Config|GetParabolicCurveSharpness) (+ (Variables|RuntimeAllocation|GetStartingHorizontalDeviation) (* (Variables|RuntimeAllocation|GetHorizontalDisplacementPerCycle) (Math|Conversions|ToFloat(Integer) (Variables|Default|GetUpdateIteration)))) 2.0) -1.0))) (* (Transformation|GetActorRightVector (Game|GetPlayerCameraManager 0)) (Variables|RuntimeAllocation|GetHorizontalDisplacementPerCycle))) false false))

(event EventBeginPlay
  ;[0 1 0 0.5] Initialization Protocols
  (bind _aswidget_scalable_text (Utilities|Casting|CastToWidget_ScalableText (UserInterface|GetUserWidgetObject (Variables|Default|GetTextWidget)))) ; Evaluates the widget class at the start before activating text display
  (Default|SetDisplayText _aswidget_scalable_text (Utilities|Text|ToText(Integer) (Variables|RuntimeAllocation|GetDamageValue)) (Variables|Default|GetTextColor))
  ;;[1 1 1] Sets movement constraints for the parabolic motion [y = -(a*x*x) + c]
  (Variables|RuntimeAllocation|SetStartingHorizontalDeviation (|CalculateHorizontalDeviationFromStartingPosition) :!pinned true) ; x
  (Variables|RuntimeAllocation|SetMaxHeightInWorldSpace (+ (.z (Transformation|GetActorLocation)) (|CalculateMaxVerticalDistanceFromStartingPosition))) ; z value for the world position corresponding to the vertex of the parabola
  (Variables|RuntimeAllocation|SetHorizontalDisplacementPerCycle (* (Variables|RuntimeAllocation|GetStartingHorizontalDeviation) (Variables|Default|GetMovementSpeedController) -1.0))
  (|CallParentFunction))

(event EventRunUpdateCycle
  ;[0 1 1 0.5] Updates the floating text state
  (|CallParentFunction)
  (if (>= (CallFunction|GetHorizontalDistanceCovered) (* (Math|Float|Absolute(Float) (Variables|RuntimeAllocation|GetStartingHorizontalDeviation)) 2.2))
    (Actor|DestroyActor)))

(fn ConstructionScript)

(fn ReachedPointOfMaxWidgetScale?
  (return (> (CallFunction|GetHorizontalDistanceCovered) (Math|Float|Absolute(Float) (Variables|RuntimeAllocation|GetStartingHorizontalDeviation)))))

(fn GetHorizontalDistanceCovered
  (return (* (Variables|Default|GetUpdateIteration) (Math|Float|Absolute(Float) (Variables|RuntimeAllocation|GetHorizontalDisplacementPerCycle)))))